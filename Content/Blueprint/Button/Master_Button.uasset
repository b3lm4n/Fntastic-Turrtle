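; Master_Button is a base interactable button that the player can trigger when standing near it.
; Player overlap with its Collision component shows the E prompt and enables input on the actor; ending the overlap hides the prompt and disables input.
; Pressing the Interactive input action calls Interactive only when no MasterTurttle actor exists in the world.
; The construction script writes the Text variable to the ButtonNumber label.
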(event OnComponentBeginOverlap(Collision)
  (params (OverlappedComponent :type Primitive%20Component%20Object%20Reference) (OtherActor :type Actor%20Object%20Reference) (OtherComp :type Primitive%20Component%20Object%20Reference) (OtherBodyIndex :type Integer) (bFromSweep :type Boolean) (SweepResult :type Hit%20Result%20Structure%20%28by%20ref%29))
  ;[1 1 1] Collision overlap/button visibillity/input enable
  (if (== OtherActor (Game|GetPlayerCharacter 0))
    (Rendering|SetVisibility (Variables|Default|GetE) true false)
    (Input|EnableInput (Game|GetPlayerController 0))))

(event OnComponentEndOverlap(Collision)
  (params (OverlappedComponent :type Primitive%20Component%20Object%20Reference) (OtherActor :type Actor%20Object%20Reference) (OtherComp :type Primitive%20Component%20Object%20Reference) (OtherBodyIndex :type Integer))
  ;[1 1 1] Overlap End/Button Visibillity/Disable input
  (if (== OtherActor (Game|GetPlayerCharacter 0))
    (Rendering|SetVisibility (Variables|Default|GetE) false false)
    (Input|DisableInput (Game|GetPlayerController 0))))

(event Input|ActionEvents|InputActionInteractive
  (params (Key :type Key%20Structure :default "None"))
  ;[1 1 1] InputAction Interactive
  (:Pressed
    (bind _outactors (Actor|GetAllActorsOfClass "/Game/Blueprint/Turttle/MasterTurttle.MasterTurttle_C"))
    (if (not (> (Utilities|Array|Length _outactors) 0))
      (CallFunction|Interactive))))

(fn ConstructionScript
  (Rendering|Components|TextRender|SetText (Variables|Default|GetButtonNumber) (Variables|Default|Gettext)))