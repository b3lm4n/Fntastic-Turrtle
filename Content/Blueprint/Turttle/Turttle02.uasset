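; Turttle02 is a turtle actor Blueprint that holds an end location and can be removed from the level.
; A custom event stores the EndLocation passed to it, and Finish02 destroys the actor.
; BeginPlay starts a short looping timer whose Stop event repeatedly calls ChangeSpeed with zero, apparently keeping the turtle stationary.
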(event Custom|Stop
  ;[1 1 1] Event Begin Play/ChangeSpeed
  (CallFunction|ChangeSpeed 0.0))

(event EventTick
  (params (DeltaSeconds :type Float%20%28single-precision%29))
  (|CallParentFunction DeltaSeconds) ; This node is disabled and will not be called.\nDrag off pins to build functionality.
)

(event EventTurttle02
  (params (EndLocation :type Vector :default "0, 0, 0"))
  ;[1 1 1] Find end location
  (Variables|Default|SetEndLocation EndLocation))

(event EventFinish02
  ;[1 1 1] Destroy Actor
  (Actor|DestroyActor))

(event EventBeginPlay
  ;[1 1 1] Event Begin Play/ChangeSpeed
  (|CallParentFunction)
  (Utilities|Time|SetTimerbyEvent (delegate Custom|Stop) 0.1 true))

(fn ConstructionScript
  (|CallParentFunction))