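; Turttle03 is a child Blueprint actor, apparently one turtle variant, that stores an end location and steadily adjusts its speed.
; BeginPlay starts a short looping timer whose Stop event repeatedly calls ChangeSpeed with a negative value, defined outside this graph.
; The Turttle03 event receives and saves EndLocation, and Finish03 destroys the actor.
; Tick is disabled and the construction script only calls the parent.
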(event Custom|Stop
  ;[1 1 1] Event Begin play/ Change Speed
  (CallFunction|ChangeSpeed -1.0))

(event EventTick
  (params (DeltaSeconds :type Float%20%28single-precision%29))
  (|CallParentFunction DeltaSeconds) ; This node is disabled and will not be called.\nDrag off pins to build functionality.
)

(event EventTurttle03
  (params (EndLocation :type Vector :default "0, 0, 0"))
  ;[1 1 1] Find end location
  (Variables|Default|SetEndLocation EndLocation))

(event EventFinish03
  ;[1 1 1] Destroy Actor
  (Actor|DestroyActor))

(event EventBeginPlay
  ;[1 1 1] Event Begin play/ Change Speed
  (|CallParentFunction)
  (Utilities|Time|SetTimerbyEvent (delegate Custom|Stop) 0.1 true))

(fn ConstructionScript
  (|CallParentFunction))