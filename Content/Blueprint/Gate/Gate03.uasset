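; Gate03 is a gate actor that spawns a turtle and detects when it reaches the finish.
; The Gate03 event spawns and stores the turtle, then sends the ENDLOCATION world position to every Interactive_Interface actor through Turttle03Message.
; When that stored turtle overlaps BOXCOLLISION, the gate calls Finish and sends the turtle Finish03Message.
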(event OnComponentBeginOverlap(BOXCOLLISION)
  (params (OverlappedComponent :type Primitive%20Component%20Object%20Reference) (OtherActor :type Actor%20Object%20Reference) (OtherComp :type Primitive%20Component%20Object%20Reference) (OtherBodyIndex :type Integer) (bFromSweep :type Boolean) (SweepResult :type Hit%20Result%20Structure%20%28by%20ref%29))
  (bind _turttle (Variables|Default|GetTurttle))
  ;[1 1 1] FinishEvent
  (if (== OtherActor _turttle)
    (CallFunction|Finish)
    (Class|InteractiveInterface|Finish03(Message) _turttle)))

(event EventGate03
  ;[1 1 1] ActivateGate03/TurrtleSpawn
  (bind _returnvalue (CallFunction|TurttleSpawn "/Game/Blueprint/Turttle/Turttle03.Turttle03_C"))
  (Variables|Default|SetTurttle _returnvalue)
  (bind _outactors (Actor|GetAllActorswithInterface "/Game/Blueprint/Base/Interactive_Interface.Interactive_Interface_C"))
  (for _array_element _outactors
    (Class|InteractiveInterface|Turttle03(Message) _array_element (Transformation|GetWorldLocation (Variables|Default|GetENDLOCATION)))))

(fn ConstructionScript
  (|CallParentFunction))