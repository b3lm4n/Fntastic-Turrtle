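; MasterGate is a gate Blueprint that provides the effects and spawning for turtle AI pawns.
; TurttleSpawn plays a spawn particle and 2D sound at the gate, spawns AI of the given pawn class at its transform, ignoring collision, and returns it.
; Finish plays a finish particle at the ENDLOCATION component along with a 2D sound.
; The construction script is empty.
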(fn ConstructionScript)

(fn TurttleSpawn
  (params (PawnClass :type Pawn%20Class%20Reference))
  (bind _returnvalue (Transformation|GetActorTransform))
  (bind (_location _rotation) (Math|Transform|BreakTransform _returnvalue))
  (Effects|SpawnEmitteratLocation "/Game/Particle/PS_SpawnTurttle.PS_SpawnTurttle" (Transformation|GetActorLocation))
  (Audio|SpawnSound2D "/Game/TrueAudio/SpawnSound.SpawnSound" 1.0 1.0 0.0 0)
  (bind _returnvalue_2 (AI|SpawnAIFromClass PawnClass 0 _location _rotation true 0))
  (return _returnvalue_2))

(fn Finish
  (Effects|SpawnEmitteratLocation "/Game/Particle/PS_FinishTurttle.PS_FinishTurttle" (Transformation|GetWorldLocation (Variables|Default|GetENDLOCATION)))
  (Audio|SpawnSound2D "/Game/TrueAudio/FinishSound.FinishSound" 1.0 1.0 0.0 0))